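; Player controller that implements gaze-dwell interaction with objects in the world.
; Each tick it compares the pawn's eye direction to a stored look vector, restarting a timer when the view moves beyond a small tolerance.
; A short steady gaze sets IsReallyGazing; a longer one fires a visibility line trace and calls DoSomething on the hit MVRP_InteractingObject.
; Persistent trace drawing and a debug print remain enabled.
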(event EventTick
  (params (DeltaSeconds :type Float%20%28single-precision%29))
  (bind _pawnref (Variables|Default|GetPawnRef))
  (bind _pawnref_2 (Variables|Default|GetPawnRef))
  (bind _outrotation (Actor|GetActorEyesViewPoint _pawnref))
  (bind (_outlocation _outrotation_2) (Actor|GetActorEyesViewPoint _pawnref_2))
  (bind _returnvalue (Math|Vector|GetForwardVector _outrotation))
  (Variables|Default|SetCheckTIme (+ (Variables|Default|GetCheckTIme) DeltaSeconds))
  (if (Variables|Default|GetIsGazing?)
    (Variables|Default|SetCompareVector _returnvalue)
    (if (> (Math|Vector|VectorLength (- (Variables|Default|GetLookVector) (Variables|Default|GetCompareVector))) 0.1)
      (Variables|Default|SetLookVector _returnvalue)
      (Variables|Default|SetCheckTIme 0.0)
      (else
        (Variables|Default|SetIsReallyGazing? (> (Variables|Default|GetCheckTIme) 1.5))
        (if (> (Variables|Default|GetCheckTIme) 2.7)
          (bind _outhit (Collision|LineTraceByChannel _outlocation (+ _outlocation (* (Math|Vector|GetForwardVector _outrotation_2) 2e+03)) "TraceTypeQuery1" false 0 "Persistent"))
          (bind _asmvrp_interacting_object (Utilities|Casting|CastToMVRP_InteractingObject (.HitActor (Collision|BreakHitResult _outhit))))
          (Default|DoSomething _asmvrp_interacting_object (.Location (Collision|BreakHitResult _outhit)))
          (Development|PrintString "RNRNERLKNRWEKLNREWNLKR")
          (Variables|Default|SetCheckTIme 0.0))))
    (else
      (Variables|Default|SetLookVector _returnvalue)
      ;[1 1 1] gazing turns back to normal and really gazing turns to false
      (Variables|Default|SetIsGazing? true)
      (Variables|Default|SetIsReallyGazing? false))))

(event EventBeginPlay
  (bind _asmvrp_main_character (Utilities|Casting|CastToMVRP_MainCharacter (Game|Player|GetPlayerPawn 0)))
  (Variables|Default|SetPawnRef _asmvrp_main_character))

(fn ConstructionScript)