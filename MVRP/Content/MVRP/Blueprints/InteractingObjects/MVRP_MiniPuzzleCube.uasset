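; Interactable mini puzzle cube that shifts 100 units along an axis chosen from the player's view direction.
; DoSomething finds the mesh axis most aligned with the view, then TeleportMacro applies a swept world-space offset.
; Only Y honors the view's sign; X and Z test absolute values, so effectively move only -X and +Z.
; The construction script gives each cube a randomly colored dynamic material.
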(event EventBeginPlay
  (|CallParentFunction))

(event Collision|EventActorBeginOverlap
  (params (OtherActor :type Actor%20Object%20Reference)))

(event EventDoSomething
  (params (Location :type Vector :default "0, 0, 0"))
  (bind _characterref (Variables|Default|GetCharacterRef))
  (bind _staticmesh (Variables|Default|GetStaticMesh))
  (bind _outrotation (Actor|GetActorEyesViewPoint _characterref))
  (bind _returnvalue (Math|Vector|GetForwardVector _staticmesh))
  (bind _returnvalue_2 (Math|Vector|GetUpVector _staticmesh))
  (bind _returnvalue_3 (Math|Vector|GetRightVector _staticmesh))
  (bind _returnvalue_4 (Math|Vector|GetForwardVector _outrotation))
  (bind _returnvalue_5 (Math|Vector|DotProduct _returnvalue_4 _returnvalue))
  (bind _returnvalue_6 (Math|Vector|DotProduct _returnvalue_4 _returnvalue_3))
  (bind _returnvalue_7 (Math|Vector|DotProduct _returnvalue_4 _returnvalue_2))
  (bind _returnvalue_8 (Math|Float|Absolute(Float) _returnvalue_5))
  (bind _returnvalue_9 (Math|Float|Absolute(Float) _returnvalue_6))
  (bind _returnvalue_10 (Math|Float|Absolute(Float) _returnvalue_7))
  (if (> _returnvalue_9 _returnvalue_10)
    (if (> _returnvalue_9 _returnvalue_8)
      ;[1 1 1] Right (Y)
      (if (> _returnvalue_6 0.0)
        (Utilities|TeleportMacro 0.0 1e+02 0.0)
        (else
          (Utilities|TeleportMacro 0.0 -1e+02 0.0)))
      (else
        ;[1 1 1] Forward (X)
        (if (> _returnvalue_8 0.0) :!label _label
          (Utilities|TeleportMacro -1e+02 0.0 0.0)
          (else
            (Utilities|TeleportMacro 1e+02 0.0 0.0)))))
    (elif (> _returnvalue_8 _returnvalue_10)
      (goto _label)
      (else
        ;[1 1 1] Up (Z)
        (if (> _returnvalue_10 0.0)
          (Utilities|TeleportMacro 0.0 0.0 1e+02)
          (else
            (Utilities|TeleportMacro 0.0 0.0 -1e+02)))))))

(event EventTick
  (params (DeltaSeconds :type Float%20%28single-precision%29)))

(fn ConstructionScript
  (|CallParentFunction)
  (bind _returnvalue (Rendering|Material|CreateDynamicMaterialInstance (Variables|Default|GetStaticMesh) 0 "/Game/MVRP/Asset/Materials/M_CubeColor_Inst.M_CubeColor_Inst" :!class /Script/Engine.PrimitiveComponent))
  (Variables|Default|SetDMI _returnvalue)
  (Rendering|Material|SetVectorParameterValue (Variables|Default|GetDMI) "Color" (Utilities|Struct|MakeLinearColor (Math|Random|RandomFloatinRange 0.0 0.5) (Math|Random|RandomFloatinRange 0.5 1.0) (Math|Random|RandomFloatinRange 0.0 1.0) 0.0) :!class /Script/Engine.MaterialInstanceDynamic))

(fn NewFunction0)