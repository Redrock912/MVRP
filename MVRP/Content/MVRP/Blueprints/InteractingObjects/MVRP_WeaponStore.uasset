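; MVRP_WeaponStore is an interactable store object that gives the player character bullets when they have enough resource points.
; Its DoSomething event compares the referenced character's ResourcePoint with BulletPrice, then adds one Bullet and prints a debug "Hello".
; The price is only a threshold, as no points are deducted, and CharacterRef is not assigned in these graphs.
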(event EventDoSomething
  (params (Location :type Vector :default "0, 0, 0"))
  (bind _characterref (Variables|Default|GetCharacterRef))
  (if (>= (Variables|/Game/MVRP/Blueprints/MVRP_MainCharacter.MVRP_MainCharacter_C|GetResourcePoint _characterref) (Variables|Default|GetBulletPrice))
    (Math|Integer|IncrementInt (Variables|/Game/MVRP/Blueprints/MVRP_MainCharacter.MVRP_MainCharacter_C|GetBullet _characterref)
      (:%20%20
        (Development|PrintString "Hello")))))

(event EventBeginPlay
  (|CallParentFunction))

(event Collision|EventActorBeginOverlap
  (params (OtherActor :type Actor%20Object%20Reference)))

(event EventTick
  (params (DeltaSeconds :type Float%20%28single-precision%29)))

(fn ConstructionScript
  (|CallParentFunction))