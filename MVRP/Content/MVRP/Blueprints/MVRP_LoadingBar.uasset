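; MVRP_LoadingBar is a circular progress indicator actor that displays a timed fill and destroys itself on completion.
; The construction script gives its PaperSprite a dynamic instance of MI_ProgressCircle.
; BeginPlay orients the sprite once from the player pawn's rotation with a 90-degree yaw offset.
; Tick samples FloatCurve over accumulated, multiplier-scaled time to drive the material's Alpha, destroying the actor when the value reaches one.
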(event EventBeginPlay
  (bind _returnvalue (Game|Player|GetPlayerPawn 0))
  (bind _returnvalue_2 (Transformation|GetActorRotation _returnvalue))
  ;[1 1 1] lookat player
  (bind _asmvrp_player_controller (Utilities|Casting|CastToMVRP_PlayerController (Game|GetPlayerController 0)))
  (Variables|Default|SetPlayerControllerRef _asmvrp_player_controller)
  (Transformation|SetWorldRotation (Variables|Default|GetPaperSprite) (Math|Rotator|MakeRotator (.roll _returnvalue_2) (.pitch _returnvalue_2) (+ (.yaw _returnvalue_2) 9e+01)) false false))

(event EventTick
  (params (DeltaSeconds :type Float%20%28single-precision%29))
  ;[1 1 1] ProgressBar
  (bind _output_get (Variables|Default|SetPanningTime (+ DeltaSeconds (Variables|Default|GetPanningTime))))
  (Rendering|Material|SetScalarParameterValue (Variables|Default|GetDMIRef) "Alpha" (Math|Curves|GetFloatValue (Variables|Default|GetFloatCurve) (* (Variables|Default|GetTimeMultiplier) _output_get)) :!class /Script/Engine.MaterialInstanceDynamic)
  (if (Math|Float|NearlyEqual(Float) (Math|Curves|GetFloatValue (Variables|Default|GetFloatCurve) (* (Variables|Default|GetTimeMultiplier) _output_get)) 1.0 1e-06)
    (Actor|DestroyActor)))

(fn ConstructionScript
  (bind _returnvalue (Rendering|Material|CreateDynamicMaterialInstance (Variables|Default|GetPaperSprite) 0 "/Game/MVRP/Asset/Materials/MI_ProgressCircle.MI_ProgressCircle" :!class /Script/Engine.PrimitiveComponent))
  (Variables|Default|SetDMIRef _returnvalue))