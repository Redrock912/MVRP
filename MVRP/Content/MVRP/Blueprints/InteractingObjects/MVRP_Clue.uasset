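; MVRP_Clue is an interactable clue object that shows a numbered clue popup in front of the player.
; DoSomething creates the popup for its ClueNumber, places it along the character's view direction, sets it to the negated view rotation and unhides it.
; The widget starts hidden, and Tick hides it again once a dot product shows the view no longer opposes the widget's forward vector.
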(event EventBeginPlay
  (|CallParentFunction)
  (Development|SetHiddeninGame (Variables|Default|GetWidget) true false))

(event Collision|EventActorBeginOverlap
  (params (OtherActor :type Actor%20Object%20Reference)))

(event EventTick
  (params (DeltaSeconds :type Float%20%28single-precision%29))
  (if (> (Math|Vector|DotProduct (Math|Vector|GetForwardVector (.OutRotation (Actor|GetActorEyesViewPoint (Variables|Default|GetCharacterRef)))) (Math|Vector|GetForwardVector (Variables|Default|GetWidget))) -0.2)
    (Development|SetHiddeninGame (Variables|Default|GetWidget) true false)))

(event EventDoSomething
  (params (Location :type Vector :default "0, 0, 0"))
  (bind _widget (Variables|Default|GetWidget))
  (bind _characterref (Variables|Default|GetCharacterRef))
  (bind (_outlocation _outrotation) (Actor|GetActorEyesViewPoint _characterref))
  (bind _returnvalue (UserInterface|CreateWidget "/Game/MVRP/Blueprints/Widget/MVRP_WB_CluePopup.MVRP_WB_CluePopup_C" 0 (Variables|Default|GetClueNumber)))
  (UserInterface|SetWidget _widget _returnvalue)
  (Transformation|SetWorldLocation _widget (+ _outlocation (* (Math|Vector|GetForwardVector _outrotation) 3.5e+02)) false false)
  (Transformation|SetWorldRotation _widget (* _outrotation -1.0) false false)
  (Development|SetHiddeninGame (Variables|Default|GetWidget) false false))

(fn ConstructionScript
  (|CallParentFunction))