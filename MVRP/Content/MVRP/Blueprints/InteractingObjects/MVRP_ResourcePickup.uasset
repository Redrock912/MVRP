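; MVRP_ResourcePickup is an interactable that opens a timed window in which the character earns resource points by looking around.
; DoSomething toggles CanEarnResource; enabling starts a looping EarnMoney timer and spawns a numbered clue popup in front of the view.
; EarnMoney awards a point whenever view yaw and pitch move far enough from the last stored sample.
; After a delay, the timer stops and the popup is destroyed, leaving the flag set.
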(event EventBeginPlay
  (|CallParentFunction))

(event Collision|EventActorBeginOverlap
  (params (OtherActor :type Actor%20Object%20Reference)))

(event EventDoSomething
  (params (Location :type Vector :default "0, 0, 0"))
  (bind _characterref (Variables|Default|GetCharacterRef))
  (bind _characterref_2 (Variables|Default|GetCharacterRef))
  (bind (_outlocation _outrotation) (Actor|GetActorEyesViewPoint _characterref_2))
  (if (Variables|/Game/MVRP/Blueprints/MVRP_MainCharacter.MVRP_MainCharacter_C|GetCanEarnResource? _characterref)
    (Variables|/Game/MVRP/Blueprints/MVRP_MainCharacter.MVRP_MainCharacter_C|SetCanEarnResource? _characterref false)
    (Utilities|Time|ClearTimerbyFunctionName 0 "EarnMoney")
    (else
      (Variables|/Game/MVRP/Blueprints/MVRP_MainCharacter.MVRP_MainCharacter_C|SetCanEarnResource? _characterref true)
      (Utilities|Time|SetTimerbyFunctionName 0 "EarnMoney" 0.1 true)
      (bind _returnvalue (Game|SpawnActorfromClass "/Game/MVRP/Blueprints/PopupObjects/MVRP_CluePopup.MVRP_CluePopup_C" (Math|Transform|MakeTransform (+ (* (Math|Vector|GetForwardVector _outrotation) 2e+02) _outlocation) _outrotation "1,1,1") "Undefined" 0 (Variables|Default|GetClueNumber) 0))
      (Variables|Default|SetCluePopup _returnvalue)
      ;[1 1 1] Earn money for some time
      (Utilities|FlowControl|Delay 5.0)
      (Utilities|Time|ClearTimerbyFunctionName 0 "EarnMoney")
      (Actor|DestroyActor (Variables|Default|GetCluePopup)))))

(event EventTick
  (params (DeltaSeconds :type Float%20%28single-precision%29)))

(fn ConstructionScript
  (|CallParentFunction))

(fn EarnMoney
  (bind _characterref (Variables|Default|GetCharacterRef))
  (bind _outrotation (Actor|GetActorEyesViewPoint _characterref))
  (if (and (== (Variables|Default|GetTempX) 0.0) (== (Variables|Default|GetTempY) 0.0))
    ;[1 1 1] Set the first value
    (Variables|Default|SetTempX (.yaw _outrotation))
    (Variables|Default|SetTempY (.pitch _outrotation))
    (else
      (LocalVariables|SetLocalX (.yaw _outrotation))
      (LocalVariables|SetLocalY (.pitch _outrotation))
      (if (> (Math|Float|Sqrt (+ (Math|Float|Power (Math|Float|Absolute(Float) (- (Variables|Default|GetTempX) (LocalVariables|GetLocalX))) 2.0) (Math|Float|Power (Math|Float|Absolute(Float) (- (LocalVariables|GetLocalY) (Variables|Default|GetTempY))) 2.0))) 7e+01)
        (bind _result (Math|Integer|IncrementInt (Variables|/Game/MVRP/Blueprints/MVRP_MainCharacter.MVRP_MainCharacter_C|GetResourcePoint (Variables|Default|GetCharacterRef)))
          (:%20%20
            (Variables|Default|SetTempX (LocalVariables|GetLocalX))
            (Variables|Default|SetTempY (LocalVariables|GetLocalY))
            (Development|PrintString (Utilities|String|ToString(Integer) _result))))))))