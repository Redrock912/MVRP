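; MVRP_NumberCube is an interactable cube that displays its Number and can be picked up by the character.
; Construction creates a dynamic instance of M_BoxNumber_Inst, and BeginPlay converts Number into U/V scroll parameters, treating the texture as a three-column number grid.
; DoSomething checks the character's HoldingObject, then snaps the cube to the character at Arrow and records it as held.
; An unconnected cube-spawning branch never runs.
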(event EventBeginPlay
  (bind _number (Variables|Default|GetNumber))
  (bind _dmi (Variables|Default|GetDMI))
  (bind _returnvalue (/ _number 3))
  (bind _returnvalue_2 (Math|Integer|%(Integer) _number 3))
  (|CallParentFunction)
  (Variables|Default|SetU_Tiling (- _returnvalue_2 1))
  (if (== _returnvalue_2 0)
    (Variables|Default|SetV_Tiling (- _returnvalue 1))
    (else
      (Variables|Default|SetV_Tiling _returnvalue)))
  (Rendering|Material|SetScalarParameterValue _dmi "U_Scroll" (Math|Conversions|ToFloat(Integer) (Variables|Default|GetU_Tiling)) :!class /Script/Engine.MaterialInstanceDynamic)
  (Rendering|Material|SetScalarParameterValue _dmi "V_Scroll" (Math|Conversions|ToFloat(Integer) (Variables|Default|GetV_Tiling)) :!class /Script/Engine.MaterialInstanceDynamic))

(event Collision|EventActorBeginOverlap
  (params (OtherActor :type Actor%20Object%20Reference)))

(event EventTick
  (params (DeltaSeconds :type Float%20%28single-precision%29)))

(event EventDoSomething
  (params (Location :type Vector :default "0, 0, 0"))
  (bind _self self)
  (bind _characterref (Variables|Default|GetCharacterRef))
  (if (== (Variables|/Game/MVRP/Blueprints/MVRP_MainCharacter.MVRP_MainCharacter_C|GetHoldingObject (Variables|Default|GetCharacterRef)) 0)
    (Transformation|AttachActorToActor _self _characterref "Arrow" "SnapToTarget" "KeepRelative" "KeepRelative" true)
    (Variables|/Game/MVRP/Blueprints/MVRP_MainCharacter.MVRP_MainCharacter_C|SetHoldingObject _characterref _self)))

(fn ConstructionScript
  (|CallParentFunction)
  (bind _returnvalue (Rendering|Material|CreateDynamicMaterialInstance (Variables|Default|GetStaticMesh) 0 "/Game/MVRP/Asset/Materials/M_BoxNumber_Inst.M_BoxNumber_Inst" :!class /Script/Engine.PrimitiveComponent))
  (Variables|Default|SetDMI _returnvalue))