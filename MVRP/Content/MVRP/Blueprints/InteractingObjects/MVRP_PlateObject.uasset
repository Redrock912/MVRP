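; Interactable number-puzzle plate that takes the character's held number cubes and checks whether they spell the Answer string.
; DoSomething detaches the held MVRP_NumberCube, scales it and places it above the next of five slot meshes, recording it in NumberCubes.
; CheckAnswer then concatenates the cube numbers in placement order, printing as it goes, and on a match spawns an MVRP_Popup in front of the character's view.
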(event EventBeginPlay
  (|CallParentFunction)
  (Variables|Default|SetCubeArray (Utilities|Array|MakeArray (Variables|Default|GetCube) (Variables|Default|GetStaticMesh1) (Variables|Default|GetStaticMesh2) (Variables|Default|GetStaticMesh3) (Variables|Default|GetStaticMesh4))))

(event Collision|EventActorBeginOverlap
  (params (OtherActor :type Actor%20Object%20Reference)))

(event EventDoSomething
  (params (Location :type Vector :default "0, 0, 0"))
  (bind _characterref (Variables|Default|GetCharacterRef))
  (bind _holdingobject (Variables|/Game/MVRP/Blueprints/MVRP_MainCharacter.MVRP_MainCharacter_C|GetHoldingObject _characterref))
  (Utilities|IsValid _holdingobject
    (:Is%20Valid
      (bind _asmvrp_number_cube (Utilities|Casting|CastToMVRP_NumberCube _holdingobject))
      (Transformation|SetActorLocation _asmvrp_number_cube (+ (Transformation|GetWorldLocation (Utilities|Array|Get(acopy) (Variables|Default|GetCubeArray) (Variables|Default|GetLength))) "0, 0,50.000000") false false)
      (Transformation|DetachFromActor _asmvrp_number_cube "KeepWorld" "KeepRelative" "KeepWorld")
      (Transformation|SetActorScale3D _asmvrp_number_cube "2.000000,2.000000,2.000000")
      (Utilities|Array|SetArrayElem (Variables|Default|GetNumberCubes) (Variables|Default|GetLength) _asmvrp_number_cube)
      (Math|Integer|IncrementInt (Variables|Default|GetLength)
        (:%20%20
          (CallFunction|CheckAnswer))))))

(event EventTick
  (params (DeltaSeconds :type Float%20%28single-precision%29)))

(fn ConstructionScript
  (|CallParentFunction))

(fn CheckAnswer
  (bind _characterref (Variables|Default|GetCharacterRef))
  (bind (_outlocation _outrotation) (Actor|GetActorEyesViewPoint _characterref))
  (Variables|Default|SetTemp "")
  (for _array_element (Variables|Default|GetNumberCubes)
    (Utilities|IsValid _array_element
      (:Is%20Valid
        (bind _output_get (Variables|Default|SetTemp (Utilities|String|Append (Variables|Default|GetTemp) (Utilities|String|ToString(Integer) (Variables|/Game/MVRP/Blueprints/InteractingObjects/MVRP_NumberCube.MVRP_NumberCube_C|GetNumber _array_element)))))
        (Development|PrintString _output_get true true "(R=1.000000,G=0.003206,B=0.927660,A=1.000000)" 5.0))))
  (if (Utilities|Enum|Equal(Enum) (Variables|Default|GetTemp) (Variables|Default|GetAnswer))
    (Game|SpawnActorfromClass "/Game/MVRP/Blueprints/PopupObjects/MVRP_Popup.MVRP_Popup_C" (Math|Transform|MakeTransform (+ _outlocation (* (Math|Vector|GetForwardVector _outrotation) 5e+02)) _outrotation "1,1,1") "Undefined" 0 0)))