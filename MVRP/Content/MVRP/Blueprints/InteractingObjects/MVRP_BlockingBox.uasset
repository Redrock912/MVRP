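; MVRP_BlockingBox is an interactable obstacle box that the player clears by spending a bullet.
; Its DoSomething event checks the referenced character's Bullet count and, if at least one remains, decrements it and destroys the box.
; The construction script creates a dynamic material instance on the static mesh and tints it cyan.
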(event EventDoSomething
  (params (Location :type Vector :default "0, 0, 0"))
  (bind _characterref (Variables|Default|GetCharacterRef))
  (if (>= (Variables|/Game/MVRP/Blueprints/MVRP_MainCharacter.MVRP_MainCharacter_C|GetBullet _characterref) 1)
    (Math|Integer|DecrementInt (Variables|/Game/MVRP/Blueprints/MVRP_MainCharacter.MVRP_MainCharacter_C|GetBullet _characterref)
      (:%20%20
        (Actor|DestroyActor)))))

(event EventBeginPlay
  (|CallParentFunction))

(event Collision|EventActorBeginOverlap
  (params (OtherActor :type Actor%20Object%20Reference)))

(event EventTick
  (params (DeltaSeconds :type Float%20%28single-precision%29)))

(fn ConstructionScript
  (|CallParentFunction)
  (bind _returnvalue (Rendering|Material|CreateDynamicMaterialInstance (Variables|Default|GetStaticMesh) 0 "/Game/MVRP/Asset/Materials/M_CubeColor_Inst.M_CubeColor_Inst" :!class /Script/Engine.PrimitiveComponent))
  (Variables|Default|SetDMI _returnvalue)
  (Rendering|Material|SetVectorParameterValue (Variables|Default|GetDMI) "Color" "(R=0.000000,G=1.000000,B=0.954199,A=1.000000)" :!class /Script/Engine.MaterialInstanceDynamic))