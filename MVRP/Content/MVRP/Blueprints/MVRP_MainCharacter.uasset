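; Player character for gaze-based targeting, with mouse-look style yaw and pitch input.
; A looping timer line-traces from the eye view, highlighting interacting-object meshes through custom depth and tracking the current target.
; Tick reads the player controller's gazing flag, spawning one loading bar in front of the view via DoOnce and destroying it when gazing stops.
; The trace ignores that loading bar.
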(event EventBeginPlay
  (bind _asmvrp_player_controller (Utilities|Casting|CastToMVRP_PlayerController (Game|GetPlayerController 0)))
  (Variables|Default|SetControllerRef _asmvrp_player_controller)
  (Utilities|Time|SetTimerbyFunctionName 0 "Trace" 0.1 true))

(event Collision|EventActorBeginOverlap
  (params (OtherActor :type Actor%20Object%20Reference)))

(event EventTick
  (params (DeltaSeconds :type Float%20%28single-precision%29))
  (bind (_outlocation _outrotation) (Actor|GetActorEyesViewPoint))
  (if (Variables|/Game/MVRP/Blueprints/MVRP_PlayerController.MVRP_PlayerController_C|GetIsReallyGazing? (Variables|Default|GetControllerRef))
    (Utilities|FlowControl|DoOnce false :!label _label
      (:Completed
        (bind _returnvalue (Game|SpawnActorfromClass "/Game/MVRP/Blueprints/MVRP_LoadingBar.MVRP_LoadingBar_C" (Math|Transform|MakeTransform (+ (* (Math|Vector|GetForwardVector _outrotation) 1e+02) _outlocation) _outrotation "1,1,1") "Undefined" 0 false 0))
        (Variables|Default|SetLoadingBar _returnvalue)))
    (else
      (Utilities|IsValid (Variables|Default|GetLoadingBar)
        (:Is%20Valid
          (Actor|DestroyActor (Variables|Default|GetLoadingBar))
          (goto _label Reset))
        (:Is%20Not%20Valid
          (goto _label Reset))))))

(event Input|AxisEvents|InputAxisTurn
  (params (AxisValue :type Float%20%28single-precision%29))
  (Pawn|Input|AddControllerYawInput AxisValue))

(event Input|AxisEvents|InputAxisLookUp
  (params (AxisValue :type Float%20%28single-precision%29))
  (Pawn|Input|AddControllerPitchInput AxisValue))

(fn ConstructionScript)

(fn Trace
  (bind (_outlocation _outrotation) (Actor|GetActorEyesViewPoint))
  (bind _outhit (Collision|LineTraceByChannel _outlocation (+ (* (Math|Vector|GetForwardVector _outrotation) 2e+03) _outlocation) "TraceTypeQuery1" false (Utilities|Array|MakeArray (Variables|Default|GetLoadingBar)) "None"))
  (bind _asmvrp_interacting_object (Utilities|Casting|CastToMVRP_InteractingObject (.HitActor (Collision|BreakHitResult _outhit)))
    (:then
      (if (not (== (Variables|Default|GetCurrentTarget) (Variables|/Game/MVRP/Blueprints/InteractingObjects/MVRP_InteractingObject.MVRP_InteractingObject_C|GetStaticMesh _asmvrp_interacting_object)))
        (Utilities|IsValid (Variables|Default|GetCurrentTarget)
          (:Is%20Valid
            ;[1 1 1] 오브젝트 끼리 겹쳐있는 경우 highlight가 남는 경우를 위한 방지용
            (Rendering|SetRenderCustomDepth (Variables|Default|GetCurrentTarget) false))
          (:Is%20Not%20Valid
            (Variables|Default|SetCurrentTarget (Variables|/Game/MVRP/Blueprints/InteractingObjects/MVRP_InteractingObject.MVRP_InteractingObject_C|GetStaticMesh _asmvrp_interacting_object))
            (Rendering|SetRenderCustomDepth (Variables|Default|GetCurrentTarget) true)
            (Variables|Default|SetIsTargetSame? true)))))
    (:CastFailed
      ;[1 1 1] 오브젝트가 없다면 highlight을 다 지운다
      (Utilities|IsValid (Variables|Default|GetCurrentTarget)
        (:Is%20Valid
          (Rendering|SetRenderCustomDepth (Variables|Default|GetCurrentTarget) false)
          (Variables|Default|SetCurrentTarget 0)
          (Variables|Default|SetIsTargetSame? false))))))